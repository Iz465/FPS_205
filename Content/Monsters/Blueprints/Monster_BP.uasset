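; Monster character Blueprint that provides melee attack, weapon wielding, patrol route and movement speed actions.
; Attack plays a punch montage and fires OnAttackEnd on completion or interruption, while the K key plays a combo punch montage.
; WieldWeapon spawns a gun on the right-hand socket, and SetMovementSpeed maps a speed state to walk speed.
; ChasePlayer is empty, with its old move-then-attack loop left disconnected.
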(event `self.ReceiveBeginPlay`)

(event `ChasePlayer`)

(event `Attack`
  (`KismetSystemLibrary.PrintString` "Attack Triggered")
  (`|PlayMontage` (`self.Mesh`) "/Game/Monsters/Animations/Goblin/Montage_MeleePunch.Montage_MeleePunch"
    (:`OnCompleted`
      _)
    (:`OnInterrupted`
      _))
  (`self.OnAttackEnd`))

(event `Key|K`
  (params (Key :type "Key Structure"))
  (:`Pressed`
    (`AnimInstance.Montage_Play` (`SkeletalMeshComponent.GetAnimInstance` (`self.Mesh`)) "/Game/Monsters/Animations/Goblin/Montage_ComboPunch.Montage_ComboPunch" 1.0 "MontageLength" 0.0 true)))

(event `WieldWeapon`
  (bind _returnvalue (`|SpawnActorFromClass` "/Game/Monsters/Weapons/BP_Gun.BP_Gun_C" (`self.GetTransform`) "Undefined" "MultiplyWithRoot" null null))
  (`self.K2_AttachToComponent` _returnvalue (`self.Mesh`) "RightHand_Weapon_Socket" "SnapToTarget" "SnapToTarget" "SnapToTarget" true)
  (set `self.isWieldingWeapon` true))

(fn `GetPatrolRoute`
  (returns (PatrolRoute :type "/Game/Monsters/AI/BP_PatrolRoute Object Reference"))
  (return (`self.PatrolRoute`)))

(fn `SetMovementSpeed`
  (params (Speed :type "/Game/Monsters/AI/Enums/E_MovementSpeed Enum" :default "NewEnumerator0"))
  (returns (SpeedValue :type "Float (double-precision)"))
  (bind _output_get (set `CharacterMovementComponent.MaxWalkSpeed` (select `/Game/Monsters/AI/Enums/E_MovementSpeed` Speed :`NewEnumerator1` 100.0 :`NewEnumerator2` 300.0 :`NewEnumerator3` 500.0 :!type "Float (single-precision)") (`self.CharacterMovement`)))
  (return _output_get))

(fn `UserConstructionScript`)